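; AC_Chat_PC is a player controller component that provides multiplayer text chat.
; On BeginPlay it creates the chat UI for the local controller and keeps a reference to its chat box.
; Enter focuses the chat box and the mouse wheel scrolls it.
; Messages pass through a server event that loops over the PlayerArray and relays them to each controller's component, whose owning-client event adds them to the box.
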(event `self.ReceiveBeginPlay`
  ;[0 1 0.2031] Create Chat
  (if (`Controller.IsLocalController` (cast `PlayerController` (`self.GetOwner`) :!pure true))
    (bind _returnvalue (`|CreateWidget` "/Game/Dynamic/TZ_/Chat/WB_ChatUI.WB_ChatUI_C"))
    (bind _output_get (set `self.chatui_ref` _returnvalue))
    (`UserWidget.AddToViewport` _output_get 0)
    (set `self.chatbox_ref` (`/Game/Dynamic/TZ_/Chat/WB_ChatUI.WB_ChatBox` _output_get))))

(event `Key|Enter`
  (params (Key :type "Key Structure"))
  ;[0 0.6953 1] Focus
  (:`Pressed`
    (`/Game/Dynamic/TZ_/Chat/WB_ChatBox.FocusChat` (`self.chatbox_ref`))))

(event `Key|MouseScrollUp`
  (params (Key :type "Key Structure"))
  ;[0.3828 0 1] Up\Down
  (:`Pressed`
    (`/Game/Dynamic/TZ_/Chat/WB_ChatBox.Scroll` (`self.chatbox_ref`) true)))

(event `Key|MouseScrollDown`
  (params (Key :type "Key Structure"))
  ;[0.3828 0 1] Up\Down
  (:`Released`
    (`/Game/Dynamic/TZ_/Chat/WB_ChatBox.Scroll` (`self.chatbox_ref`) false)))

(event `SendChatMessage_OnServer`
  (params (MessageString :type String))
  ;[0 0.7891 1] Server
  (for _array_element (`GameStateBase.PlayerArray` (`GameplayStatics.GetGameState`))
    (`self.SendChatMessage_OnOwningClient` (`Actor.K2_GetComponentsByClass` (`PlayerState.GetPlayerController` _array_element) "AC_Chat_PC_C") MessageString)))

(event `SendChatMessage_OnOwningClient`
  (params (MessageString :type String))
  ;[0.07812 1 0] Client
  (`/Game/Dynamic/TZ_/Chat/WB_ChatBox.Add Chat Message` (`self.chatbox_ref`) MessageString))